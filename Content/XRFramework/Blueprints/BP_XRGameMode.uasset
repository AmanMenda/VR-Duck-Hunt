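; BP_XRGameMode runs the rules of an XR duck-shooting game, tracking score and remaining chances.
; StartGame resets both values, updates the BP_XRPawn display and tells every BP_DuckSpawner to start spawning.
; DuckKilled adds score and DuckEscaped removes a chance, each then checking game over, which shows the pawn's game-over display and stops the spawners.
; RestartGame destroys the pawn's weapons before starting again.
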(event EventTick
  (params (DeltaSeconds :type Float%20%28single-precision%29)))

(event EventBeginPlay
  (Variables|Default|SetScore 0)
  (Variables|Default|SetChances 3))

(fn ConstructionScript)

(fn RestartGame
  (bind _xrpawn (CallFunction|GetXRPawn))
  (Default|DestroyWeapons _xrpawn)
  (CallFunction|StartGame))

(fn GetXRPawn
  (bind _asbp_xrpawn (Utilities|Casting|CastToBP_XRPawn (Game|Player|GetPlayerPawn 0))
    (:then
      _)
    (:CastFailed
      _))
  (return _asbp_xrpawn))

(fn StartGame
  (Variables|Default|SetScore 0)
  (Variables|Default|SetChances 3)
  (bind _xrpawn (CallFunction|GetXRPawn))
  (Default|ShowScore _xrpawn)
  (Default|UpdateScore _xrpawn)
  (Default|UpdateChances _xrpawn 3)
  (bind _outactors (Actor|GetAllActorsOfClass "/Game/XRFramework/Blueprints/CustomBP/BP_DuckSpawner.BP_DuckSpawner_C"))
  (Default|StartSpawning _outactors))

(fn DuckKilled
  (bind _output_get (Variables|Default|SetScore (+ (Variables|Default|GetScore) 10)))
  (bind _xrpawn (CallFunction|GetXRPawn))
  (Default|UpdateScore _xrpawn _output_get)
  (CallFunction|CheckGameOver))

(fn CheckGameOver
  (if (<= (Variables|Default|GetChances) 0)
    (bind _xrpawn (CallFunction|GetXRPawn))
    (Utilities|IsValid _xrpawn
      (:Is%20Valid
        (Default|ShowGameOver _xrpawn)
        (bind _outactors (Actor|GetAllActorsOfClass "/Game/XRFramework/Blueprints/CustomBP/BP_DuckSpawner.BP_DuckSpawner_C"))
        (Default|StopSpawning _outactors)))))

(fn DuckEscaped
  (bind _output_get (Variables|Default|SetChances (- (Variables|Default|GetChances) 1)))
  (bind _xrpawn (CallFunction|GetXRPawn))
  (Utilities|IsValid _xrpawn
    (:Is%20Valid
      (Default|UpdateChances _xrpawn _output_get)
      (CallFunction|CheckGameOver))))