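; BP_DuckMover is a moving duck target that travels from its spawn point to a target location and can be shot by projectiles.
; Each tick it advances along a straight lerp at constant speed, adding a sine-wave vertical bob, and destroys itself on arrival or if the path is negligibly short.
; Overlap with a BP_Projectile plays a pitch-randomised hit sound and destroys it.
; An older constant-speed interp movement is left unconnected.
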(event EventBeginPlay
  (bind _output_get (Variables|Default|SetStartLocation (Transformation|GetActorLocation)))
  (bind _output_get_2 (Variables|Default|SetPathLength (Math|Vector|VectorLength (- _output_get (Variables|Default|GetTargetLocation)))))
  (if (< _output_get_2 1.0)
    (Actor|DestroyActor)))

(event Collision|EventActorBeginOverlap
  (params (OtherActor :type Actor%20Object%20Reference))
  (bind _asbp_projectile (Utilities|Casting|CastToBP_Projectile OtherActor))
  (Audio|PlaySoundatLocation "/Game/XRFramework/Audio/Hit.Hit" (Transformation|GetActorLocation) "0, 0, 0" 1.0 (Math|Random|RandomFloatinRange 0.9 1.1) 0.0 0 0 _asbp_projectile 0)
  (Actor|DestroyActor))

(event EventTick
  (params (DeltaSeconds :type Float%20%28single-precision%29))
  (Variables|Default|SetPathAlpha (+ (Variables|Default|GetPathAlpha) (/ (* (Utilities|Time|GetWorldDeltaSeconds) (Variables|Default|GetMoveSpeed)) (Variables|Default|GetPathLength))))
  (Transformation|SetActorLocation (+ (Math|Vector|MakeVector 0.0 0.0 (* (Math|Trig|Sin(Radians) (* (* (Variables|Default|GetPathAlpha) (Variables|Default|GetOscillationFreq)) 6.2832)) (Variables|Default|GetArcHeight))) (Math|Vector|Lerp(Vector) (Variables|Default|GetStartLocation) (Variables|Default|GetTargetLocation) (Variables|Default|GetPathAlpha))) false false)
  (if (>= (Variables|Default|GetPathAlpha) 1.0)
    (Actor|DestroyActor)))

(fn ConstructionScript)